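; Orthographic RTS-style camera that takes over player 0's view on BeginPlay, then pans and zooms across the scene.
; Each tick, MoveCamera combines keyboard input with mouse edge scrolling, rotates it by the spring arm's yaw and offsets the root.
; The mouse wheel drives a clamped zoom level that sets ortho width.
; The movement-direction math also scales pan speed by zoom, slowing as the view zooms in.
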(event `self.ReceiveBeginPlay`
  ;[1 1 1 0.5] Apply View
  (`PlayerController.SetViewTargetWithBlend` (`GameplayStatics.GetPlayerController` 0) self 0.0 "VTBlend_Linear" 0.0 false))

(event `self.ReceiveTick`
  (params (DeltaSeconds :type "Float (single-precision)"))
  ;[0 0.15 1 0.5] Movement
  (`self.MoveCamera`))

(event `InputAxisKey|MouseWheelAxis`
  (params (AxisValue :type "Float (single-precision)"))
  ;[0 0.15 1 0.5] Zoom
  (bind _output_get (set `self.CurrentZoom` (`KismetMathLibrary.FClamp` (+ AxisValue (`self.CurrentZoom`)) 0.0 10.0)))
  (`self.ChangeZoom` _output_get))

(fn `ChangeZoom`
  (params (ZoomValue :type "Float (double-precision)"))
  (`CameraComponent.SetOrthoWidth` (`self.Camera`) (+ (* (- 1.0 (`KismetMathLibrary.NormalizeToRange` ZoomValue 0.0 10.0)) 6000.0) 1500.0)))

(fn `MoveCamera`
  (locals (mousePos :type "Vector2D Structure"))
  (bind (_returnvalue_x _returnvalue_y) (`KismetMathLibrary.BreakVector2D` (`WidgetLayoutLibrary.GetViewportSize`)))
  (bind _returnvalue (`WidgetLayoutLibrary.GetViewportScale`))
  (bind (_mousepos_x _mousepos_y) (`KismetMathLibrary.BreakVector2D` (`local.mousePos`)))
  (bind (_relativerotation_roll _relativerotation_pitch _relativerotation_yaw) (`KismetMathLibrary.BreakRotator` (`SceneComponent.RelativeRotation` (`self.SpringArm`))))
  ;[1 1 1 0.5] Get Mouse Position on Viewport
  (bind _returnvalue_2 (`WidgetLayoutLibrary.GetMousePositionOnViewport`))
  (set `local.mousePos` (* _returnvalue_2 (`KismetMathLibrary.MakeVector2D` _returnvalue _returnvalue)))
  ;[1 1 1 0.5] Get Movement Direction
  (bind _output_get (set `self.CameraMovement` (`KismetMathLibrary.MakeVector2D` (`self.Get Movement Direction` (* (`self.GetInputAxisValue`) -1.0) _mousepos_x _returnvalue_x) (`self.Get Movement Direction` (`self.GetInputAxisValue`) _mousepos_y _returnvalue_y))))
  ;[1 1 1 0.5] Apply Movement
  (`SceneComponent.K2_AddRelativeLocation` (`self.DefaultSceneRoot`) (`KismetMathLibrary.GreaterGreater_VectorRotator` (`KismetMathLibrary.Conv_Vector2DToVector` _output_get) (`KismetMathLibrary.MakeRotator` 0.0 0.0 _relativerotation_yaw)) false false))

(fn `UserConstructionScript`)