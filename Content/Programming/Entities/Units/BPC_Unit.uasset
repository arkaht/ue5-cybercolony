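; Base RTS unit character that players select and right-click to move or attack, configured from UnitData for mesh, movement, health, senses and combat.
; Team decides selection priority, colors, fog-of-war behavior and player-controller registration.
; Pawn sensing and click orders (sphere overlap finds enemies) feed the Targeting component or move orders, which drive BPAIC_Unit's states.
; Death destroys the actor, returning stable resource costs for player units.
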(event `self.ReceiveBeginPlay`
  (bind _health (`self.Health`))
  (bind _selection (`self.Selection`))
  (bind _team (`self.Team`))
  (bind _selection_settings (`self.Selection Settings`))
  (bind _fogofwar (`self.FogOfWar`))
  (bind _bool (`/Game/Programming/Utils/BPFL_Game.Is Player Team` _team))
  (bind _color (`/Game/Programming/Data/Primaries/PDA_Team.Color` _team))
  (`|ExecutionSequence`
    (:`then_0`
      ;[1 1 1 0.33] Setup Components
      ;;[1 1 1 0.33] Setup Selection
      (set `/Game/Programming/Entities/Components/BPAC_Selection.Priority` (`KismetMathLibrary.SelectInt` (`/Game/Programming/Data/Primaries/PDA_SelectionSettings.Player Units Priority` _selection_settings) (`/Game/Programming/Data/Primaries/PDA_SelectionSettings.Enemy Units Priority` _selection_settings) _bool) _selection)
      (`/Game/Programming/Entities/Components/BPAC_Selection.Set Decal` _selection (`self.DecalSelection`) _color)
      ;;[1 1 1 0.33] Setup Health
      (`/Game/Programming/Entities/Components/BPAC_Health.Setup Widget` _health (`self.WidgetHealth`) _color)
      (`/Game/Programming/Entities/Components/BPAC_Health.Bind to Selection` _health _selection)
      ;;[1 1 1 0.33] Setup Fog Of War
      (`ActorComponent.SetActive` _fogofwar _bool false)
      (set `/Game/Programming/FoW/BPAC_FogOfWar.Can Visually Hide` (not _bool) _fogofwar))
    (:`then_1`
      ;[1 1 1 0.33] Retrieve Player Controller
      (bind _asbppc_player_controller (cast `/Game/Programming/Core/BPPC_PlayerController` (`GameplayStatics.GetPlayerController` 0)))
      (bind _output_get (set `self.Player Controller` _asbppc_player_controller))
      ;[1 1 1 0.33] Register to Player Controller
      (if _bool
        (`/Game/Programming/Core/BPPC_PlayerController.Register Unit` _output_get self)))
    (:`then_2`
      ;[1 1 1 0.33] Retrieve AI Controller
      (bind _asbpaic_unit (cast `/Game/Programming/Entities/Units/BPAIC_Unit` (`AIBlueprintHelperLibrary.GetAIController` self)))
      (set `self.BP AI Controller` _asbpaic_unit))
    (:`then_3`
      (`self.Setup Data`))))

(event `self.Selection.On Selected`)

(event `self.Selection.On Un Selected`)

(event `self.Selection.On Right Click`
  (params (Location :type "Vector Structure"))
  ;[1 1 1 0.33] Check Team
  (if (`/Game/Programming/Utils/BPFL_Game.Is Player Team` (`self.Team`))
    (`self.Order to Location` Location)))

(event `self.ReceiveEndPlay`
  (params (EndPlayReason :type "EEndPlayReason Enum" :default "Destroyed"))
  (bind _player_controller (`self.Player Controller`))
  ;[1 1 1 0.33] Un Register to Player Controller
  (`/Engine/EditorBlueprintResources/StandardMacros.IsValid` _player_controller
    (:`Is Valid`
      (`/Game/Programming/Core/BPPC_PlayerController.Un Register Unit` _player_controller self))))

(event `self.PawnSensing.OnSeePawn`
  (params (Pawn :type "Pawn Object Reference"))
  (bind _state (`/Game/Programming/Entities/Units/BPAIC_Unit.Get State` (`self.BP AI Controller`)))
  ;[1 1 1 0.33] Target Detection
  (`/Game/Programming/Entities/Components/BPAC_Targeting.Try Enemy Target` (`self.Targeting`) Pawn (`|EnumEquality` "NewEnumerator0" _state) (`|EnumEquality` "NewEnumerator1" _state)))

(event `self.Health.On Die`
  (if (`/Game/Programming/Utils/BPFL_Game.Is Player Team` (`self.Team`))
    (`/Game/Programming/Core/BPPC_PlayerController.Add Resources` (`self.Player Controller`) (`|MakeMap` "NewEnumerator0" :!type "/Game/Programming/Data/Enums/E_Consumable_Resource Enum") (`/Game/Programming/Data/Primaries/PDA_Unit.Cost Stables` (`self.Unit Data`))))
  (`self.K2_DestroyActor`))

(event `self.Targeting.On Target New`
  (params (Target :type "/Game/Programming/Entities/BPI_Entity Interface") (`Target Actor` :type "Actor Object Reference"))
  (bind _bp_ai_controller (`self.BP AI Controller`))
  (`/Game/Programming/Entities/Units/BPAIC_Unit.Set Target` _bp_ai_controller `Target Actor`)
  (`/Game/Programming/Entities/Units/BPAIC_Unit.Set State` _bp_ai_controller "NewEnumerator1"))

(event `self.Targeting.On Target Remove`
  (`/Game/Programming/Entities/Units/BPAIC_Unit.Set State` (`self.BP AI Controller`) "NewEnumerator0"))

(fn `Can Be Targeted`
  (returns (`Can Be Target` :type Boolean))
  (return true))

(fn `Get Action Classes`
  (returns (`Action Classes` :type "Array of /Game/Programming/Entities/Actions/BP_Action Class Reference"))
  (return (`/Game/Programming/Data/Primaries/PDA_Entity.Action Classes` (`self.Unit Data`))))

(fn `Get Actor`
  (returns (Actor :type "Actor Object Reference"))
  (return self))

(fn `Get Data`
  (returns (Data :type "/Game/Programming/Data/Primaries/PDA_Entity Object Reference"))
  (return (`self.Unit Data`)))

(fn `Get Health Component`
  (returns (Health :type "/Game/Programming/Entities/Components/BPAC_Health Object Reference"))
  (return (`self.Health`)))

(fn `Get Selection Component`
  (returns (SelectionComponent :type "/Game/Programming/Entities/Components/BPAC_Selection Object Reference"))
  (return (`self.Selection`)))

(fn `Get Team`
  (returns (Team :type "/Game/Programming/Data/Primaries/PDA_Team Object Reference"))
  (return (`self.Team`)))

(fn `Halt`
  (`/Game/Programming/Entities/Units/BPAIC_Unit.Set State` (`self.BP AI Controller`) "NewEnumerator0"))

(fn `Has Enemy Target`
  (returns (`Is Valid` :type Boolean))
  (return (`KismetSystemLibrary.IsValid` (`KismetSystemLibrary.Conv_InterfaceToObject` (`self.Enemy Target`)))))

(fn `Order to Location`
  (params (Location :type "Vector Structure"))
  (bind _outactors (`KismetSystemLibrary.SphereOverlapActors` Location 92.0 (`|MakeArray` "ObjectTypeQuery3" "ObjectTypeQuery2" :!type "EObjectTypeQuery Enum") "/Script/Engine.Actor"))
  (for _array_element _outactors
    (bind _asbpi_entity (cast `/Game/Programming/Entities/BPI_Entity` _array_element))
    ;[1 1 1 0.33] Check Enemy
    (bind _team (`/Game/Programming/Entities/BPI_Entity.Get Team` _asbpi_entity))
    (if (!= _team (`self.Team`))
      (`/Game/Programming/Entities/Components/BPAC_Targeting.Set Target` (`self.Targeting`) _asbpi_entity true)
      (`NiagaraFunctionLibrary.SpawnSystemAtLocation` "/Game/Art/Particle/P_Click_Enemy.P_Click_Enemy" Location)
      (return)))
  ;[1 1 1 0.33] Move To
  (`self.Set Move Location` Location)
  (`NiagaraFunctionLibrary.SpawnSystemAtLocation` "/Game/Art/Particle/P_Click.P_Click" Location))

(fn `Set Enemy Target`
  (params (Entity :type "/Game/Programming/Entities/BPI_Entity Interface"))
  (bind _bp_ai_controller (`self.BP AI Controller`))
  (bind _output_get (set `self.Enemy Target` Entity))
  (`/Engine/EditorBlueprintResources/StandardMacros.IsValid` (`KismetSystemLibrary.Conv_InterfaceToObject` _output_get)
    (:`Is Valid`
      (bind _actor (`/Game/Programming/Entities/BPI_Entity.Get Actor` _output_get))
      (`/Game/Programming/Entities/Units/BPAIC_Unit.Set Target` _bp_ai_controller _actor)
      (`/Game/Programming/Entities/Units/BPAIC_Unit.Set State` _bp_ai_controller (select `bool` (`KismetSystemLibrary.IsValid` _actor) :`false` "NewEnumerator0" :`true` "NewEnumerator1" :!type "/Game/Programming/Entities/Units/E_UnitState Enum")))))

(fn `Set Move Location`
  (params (Location :type "Vector Structure"))
  (bind _bp_ai_controller (`self.BP AI Controller`))
  (`/Game/Programming/Entities/Units/BPAIC_Unit.Move To` _bp_ai_controller Location)
  (`/Game/Programming/Entities/Units/BPAIC_Unit.Set State` _bp_ai_controller "NewEnumerator2")
  (`Controller.StopMovement` _bp_ai_controller)
  (set `self.Enemy Target` null))

(fn `Setup Data`
  (bind _mesh (`self.Mesh`))
  (bind _unit_data (`self.Unit Data`))
  (bind _bp_ai_controller (`self.BP AI Controller`))
  ;[1 1 1 0.33] Move Speed
  (set `CharacterMovementComponent.MaxWalkSpeed` (`/Game/Programming/Data/Primaries/PDA_Unit.Movement Speed` _unit_data) (`self.CharacterMovement`))
  ;[1 1 1 0.33] Mesh
  (`SkinnedMeshComponent.SetSkinnedAssetAndUpdate` _mesh (`/Game/Programming/Data/Primaries/PDA_Unit.Skeletal Mesh` _unit_data) true)
  (`SkeletalMeshComponent.SetAnimInstanceClass` _mesh (`/Game/Programming/Data/Primaries/PDA_Unit.Anim Class` _unit_data))
  ;[1 1 1 0.33] Setup STW Shader
  (`PrimitiveComponent.SetCustomDepthStencilValue` _mesh (`/Game/Programming/Data/Primaries/PDA_Team.Custom Depth Stencil Value` (`self.Team`)))
  ;[1 1 1 0.33] Set Health
  (`/Game/Programming/Entities/Components/BPAC_Health.Set Healths` (`self.Health`) (`/Game/Programming/Data/Primaries/PDA_Entity.Health` _unit_data))
  ;[1 1 1 0.33] Set Detection Range
  (set `PawnSensingComponent.SightRadius` (`/Game/Programming/Data/Primaries/PDA_Unit.Detection Range` _unit_data) (`self.PawnSensing`))
  ;[1 1 1 0.33] Set Attack Data
  (`/Game/Programming/Entities/Units/BPAIC_Unit.Set Attack Range` _bp_ai_controller (`/Game/Programming/Data/Primaries/PDA_Unit.Attack Range` _unit_data))
  (`/Game/Programming/Entities/Units/BPAIC_Unit.Set Attack Damage` _bp_ai_controller (`/Game/Programming/Data/Primaries/PDA_Unit.Damage` _unit_data))
  (`/Game/Programming/Entities/Units/BPAIC_Unit.Set Attack Cooldown` _bp_ai_controller (`/Game/Programming/Data/Primaries/PDA_Unit.Attack Cooldown` _unit_data))
  ;[1 1 1 0.33] Targeting Setup
  (set `/Game/Programming/Entities/Components/BPAC_Targeting.Team` (`self.Team`) (`self.Targeting`))
  ;[1 1 1 0.33] FoW Radius
  (set `/Game/Programming/FoW/BPAC_FogOfWar.See Radius` (`/Game/Programming/Data/Primaries/PDA_Entity.Vision Radius` _unit_data) (`self.FogOfWar`)))

(fn `Should Becomes new Target`
  (params (`Current Target` :type "/Game/Programming/Entities/BPI_Entity Interface") (`New Target` :type "/Game/Programming/Entities/BPI_Entity Interface"))
  (returns (`Has Priority` :type Boolean))
  (bind _targeting (`self.Targeting`))
  (bind (_has_priority _is_equal) (`/Game/Programming/Entities/Components/BPAC_Targeting.Check Target Priority` _targeting `New Target`))
  (if _has_priority
    (return true)
    (elif (and _is_equal (`/Game/Programming/Entities/Components/BPAC_Targeting.Is Target Prioritized` _targeting))
      (bind _has_priority_2 (`/Game/Programming/Entities/Components/BPAC_Targeting.Check Target Distance` _targeting `New Target`))
      (return _has_priority_2)
      (else
        (return false)))))

(fn `UserConstructionScript`)