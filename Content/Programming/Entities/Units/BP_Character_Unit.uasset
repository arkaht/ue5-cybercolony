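; Base Character for selectable, team-owned units, configured from UnitData and Team data.
; BeginPlay applies speed, health, mesh and animation, then colors the health widget and selection decal by team.
; The mesh takes the team's custom depth stencil value for the STW shader, and selection component events toggle the decal.
; Player-team units register with BP_PlayerController on BeginPlay, and EndPlay unregisters through that controller.
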(event `self.ReceiveBeginPlay`
  (bind _mesh (`self.Mesh`))
  (bind _unit_data (`self.Unit Data`))
  (bind _color (`/Game/Programming/Data/Primaries/PDA_Team.Color` (`self.Team`)))
  (`|ExecutionSequence`
    (:`then_0`
      ;[1 1 1 0.33] Setup Data
      (set `CharacterMovementComponent.MaxWalkSpeed` (`/Game/Programming/Data/Primaries/PDA_Unit.Movement Speed` _unit_data) (`self.CharacterMovement`))
      (bind _output_get (set `self.Health` (`/Game/Programming/Data/Primaries/PDA_Unit.Health` _unit_data)))
      ;;[1 1 1 0.33] Mesh
      (`SkinnedMeshComponent.SetSkinnedAssetAndUpdate` _mesh (`/Game/Programming/Data/Primaries/PDA_Unit.Skeletal Mesh` _unit_data) true)
      (`SkeletalMeshComponent.SetAnimInstanceClass` _mesh (`/Game/Programming/Data/Primaries/PDA_Unit.Anim Class` _unit_data))
      ;;[1 1 1 0.33] Setup STW Shader
      (`PrimitiveComponent.SetCustomDepthStencilValue` _mesh (`/Game/Programming/Data/Primaries/PDA_Team.Custom Depth Stencil Value` (`self.Team`))))
    (:`then_1`
      ;[1 1 1 0.33] Get WBP Health
      (bind _aswbp_health (cast `/Game/Programming/UI/WBP_Health` (`WidgetComponent.GetWidget` (`self.WidgetHealth`))))
      (bind _output_get_2 (set `self.WBP Health` _aswbp_health))
      ;;[1 1 1 0.33] Setup Variables
      (set `/Game/Programming/UI/WBP_Health.Health` (`self.Health`) _output_get_2)
      (set `/Game/Programming/UI/WBP_Health.Max Health` _output_get _output_get_2)
      (set `/Game/Programming/UI/WBP_Health.Color` _color _output_get_2))
    (:`then_2`
      ;[1 1 1 0.33] Setup Decal Selection Material
      (bind _returnvalue (`KismetMaterialLibrary.CreateDynamicMaterialInstance` "/Game/Art/Units/M_Decal_UnitSelection.M_Decal_UnitSelection"))
      (`MaterialInstanceDynamic.SetVectorParameterValue` _returnvalue "Color" _color)
      (`DecalComponent.SetDecalMaterial` (`self.DecalSelection`) _returnvalue))
    (:`then_3`
      ;[1 1 1 0.33] Retrieve Player Controller
      (bind _asbp_player_controller (cast `/Game/Programming/Core/BP_PlayerController` (`GameplayStatics.GetPlayerController` 0)))
      (bind _output_get_3 (set `self.BP Player Controller` _asbp_player_controller))
      ;[1 1 1 0.33] Register to Player Controller
      (if (`self.Is Player Team`)
        (`/Game/Programming/Core/BP_PlayerController.Register Unit` _output_get_3 self)))))

(event `self.BP_Selection.OnSelected`
  ;[1 1 1 0.33] Show Selection Decal
  (`SceneComponent.SetVisibility` (`self.DecalSelection`) true false))

(event `self.BP_Selection.OnUnselected`
  ;[1 1 1 0.33] Hide Selection Decal
  (`SceneComponent.SetVisibility` (`self.DecalSelection`) false false))

(event `self.ReceiveEndPlay`
  (params (EndPlayReason :type "EEndPlayReason Enum" :default "Destroyed"))
  (bind _bp_player_controller (`self.BP Player Controller`))
  ;[1 1 1 0.33] Un Register to Player Controller
  (`/Engine/EditorBlueprintResources/StandardMacros.IsValid` _bp_player_controller
    (:`Is Valid`
      (`/Game/Programming/Core/BP_PlayerController.Un Register Unit` _bp_player_controller self))))

(fn `GetActor`
  (returns (Actor :type "Actor Object Reference"))
  (return self))

(fn `GetSelectionComponent`
  (returns (SelectionComponent :type "/Game/Programming/Entities/BPAC_Selection Object Reference"))
  (return (`self.BP_Selection`)))

(fn `Is Player Team`
  (returns (Bool :type Boolean))
  (return (== (`self.Team`) "/Game/Design/Data/Teams/DA_Team_Player.DA_Team_Player")))

(fn `UserConstructionScript`)