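; BP_Building is a building actor that spawns in placement mode, previewing validity with green or red materials.
; Begin and end overlap events track blocking actors, turning the preview red and flagging placement as blocked until none remain.
; Place fails if blocked or if the player controller lacks any build cost resource.
; Otherwise it consumes the cost, restores the base material and switches collision to OverlapVisibility.
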(event `self.ReceiveBeginPlay`
  ;[1 1 1] Initialization
  (bind _returnvalue (`MaterialInterface.GetBaseMaterial` (`PrimitiveComponent.GetMaterial` (`self.Cube`) 0)))
  (set `self.BaseMat` _returnvalue)
  (`PrimitiveComponent.SetMaterial` (`self.Cube`) 0 (`self.GreenPlacementMat`))
  (set `self.inPlacement` true))

(event `self.ReceiveActorBeginOverlap`
  (params (OtherActor :type "Actor Object Reference"))
  ;[1 1 1] Blocking Detection
  (if (`self.inPlacement`)
    (`KismetArrayLibrary.Array_Add` (`self.blockingActors`) OtherActor)
    (set `self.placementBlocked` true)
    (`PrimitiveComponent.SetMaterial` (`self.Cube`) 0 (`self.RedPlacementMat`))))

(event `self.ReceiveActorEndOverlap`
  (params (OtherActor :type "Actor Object Reference"))
  ;[1 1 1] Blocking Detection
  (if (`self.inPlacement`)
    (`KismetArrayLibrary.Array_RemoveItem` (`self.blockingActors`) OtherActor)
    (if (== (`KismetArrayLibrary.Array_Length` (`self.blockingActors`)) 0)
      (set `self.placementBlocked` false)
      (`PrimitiveComponent.SetMaterial` (`self.Cube`) 0 (`self.GreenPlacementMat`)))))

(fn `GetActor`
  (returns (Actor :type "Actor Object Reference"))
  (return null))

(fn `GetSelectionComponent`
  (returns (SelectionComponent :type "/Game/Programming/Entities/BPAC_Selection Object Reference"))
  (return null))

(fn `Place`
  (returns (Sucess :type Boolean))
  (if (not (`self.placementBlocked`))
    (bind _sucess (`self.PlayerHasResources`))
    (if _sucess
      (bind _asbp_player_controller (cast `/Game/Programming/Core/BP_PlayerController` (`GameplayStatics.GetPlayerController` 0)))
      (`/Game/Programming/Core/BP_PlayerController.ConsumeResources` _asbp_player_controller (`/Game/Programming/Data/Primaries/PDA_Building.BuildCost` (`self.BuildingDatas`)))
      (`PrimitiveComponent.SetMaterial` (`self.Cube`) 0 (`self.BaseMat`))
      (set `self.inPlacement` false)
      (`PrimitiveComponent.SetCollisionProfileName` (`self.Cube`) "OverlapVisibility" true)
      (return true)
      (else
        _)))
  (return false))

(fn `PlayerHasResources`
  (returns (sucess :type Boolean))
  (bind (_buildcost_iron _buildcost_copper _buildcost_gold _buildcost_flux _buildcost_population _buildcost_food _buildcost_energy) (break `/Game/Programming/Data/Structures/S_Resources` (`/Game/Programming/Data/Primaries/PDA_Building.BuildCost` (`self.BuildingDatas`))))
  (bind _asbp_player_controller (cast `/Game/Programming/Core/BP_PlayerController` (`GameplayStatics.GetPlayerController` 0)))
  (bind (_playerresources_iron _playerresources_copper _playerresources_gold _playerresources_flux _playerresources_population _playerresources_food _playerresources_energy) (break `/Game/Programming/Data/Structures/S_Resources` (`/Game/Programming/Core/BP_PlayerController.PlayerResources` _asbp_player_controller)))
  (if (> _buildcost_iron _playerresources_iron)
    (return false)
    (elif (> _buildcost_copper _playerresources_copper)
      (return false)
      (elif (> _buildcost_gold _playerresources_gold)
        (return false)
        (elif (> _buildcost_flux _playerresources_flux)
          (return false)
          (elif (> _buildcost_population _playerresources_population)
            (return false)
            (elif (> _buildcost_food _playerresources_food)
              (return false)
              (elif (> _buildcost_energy _playerresources_energy)
                (return false)
                (else
                  (return true))))))))))

(fn `UserConstructionScript`)