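; Entity action that produces a unit from a Nexus, using its UnitData.
; Initialize casts the owning entity's actor to BPP_Nexus and caches it.
; CanAct checks that the Nexus's player controller has the unit's consumable and stable resource costs.
; DoAction has the game mode spawn the unit at the Nexus spawn point for its team, consuming resources only if the spawn succeeds.
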(fn `Can Act`
  (returns (`Can Act` :type Boolean))
  (bind _unit_data (`self.Unit Data`))
  (bind _nexus (`self.Nexus`)
    (:`then`
      (return (`/Game/Programming/Core/BPPC_PlayerController.Has Resources` (`/Game/Programming/Entities/Buildings/BPA_Building.Player Controller` _nexus) (`/Game/Programming/Data/Primaries/PDA_Unit.Cost Consumables` _unit_data) (`/Game/Programming/Data/Primaries/PDA_Unit.Cost Stables` _unit_data))))
    (:`else`
      (return false))))

(fn `Do Action`
  (bind _unit_data (`self.Unit Data`))
  (bind _nexus (`self.Nexus`)
    (:`then`
      (bind (_returnvalue_location _returnvalue_rotation) (`KismetMathLibrary.BreakTransform` (`SceneComponent.K2_GetComponentToWorld` (`/Game/Programming/Entities/Buildings/BPP_Nexus.Spawn Point` _nexus))))
      (bind _returnvalue (`/Game/Programming/Core/BPG_Gamemode.Spawn Unit` (`/Game/Programming/Entities/Buildings/BPA_Building.Gamemode` _nexus) (`KismetMathLibrary.MakeTransform` _returnvalue_location _returnvalue_rotation) _unit_data (`/Game/Programming/Entities/Buildings/BPA_Building.Team` _nexus)))
      (`/Engine/EditorBlueprintResources/StandardMacros.IsValid` _returnvalue
        (:`Is Valid`
          (`/Game/Programming/Core/BPPC_PlayerController.Consume Resources` (`/Game/Programming/Entities/Buildings/BPA_Building.Player Controller` _nexus) (`/Game/Programming/Data/Primaries/PDA_Unit.Cost Consumables` _unit_data) (`/Game/Programming/Data/Primaries/PDA_Unit.Cost Stables` _unit_data)))))
    (:`else`)))

(fn `Initialize`
  (bind _actor (`/Game/Programming/Entities/BPI_Entity.Get Actor` (`self.Entity`)))
  (bind _asbpp_nexus (cast `/Game/Programming/Entities/Buildings/BPP_Nexus` _actor))
  (set `self.Nexus` _asbpp_nexus))