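; BP_Action_Toggle is an entity action that pauses and resumes an entity by toggling tick on its Actor.
; On initialize it caches the Actor from the Entity and shows RunImage on the action button if tick is already disabled.
; Each activation checks the Actor is valid, flips its tick state and swaps the button texture between Image and RunImage to match.
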(fn `Do Action`
  (bind _actor (`self.Actor`)
    (:`then`
      (bind _returnvalue (`Actor.IsActorTickEnabled` _actor))
      (`Actor.SetActorTickEnabled` _actor (not _returnvalue))
      (`/Game/Programming/UI/WBP_ATH_ActionButton.Set Texture` (`self.Action Button`) (select `bool` _returnvalue :`false` (`self.Run Image`) :`true` (`self.Image`))))
    (:`else`)))

(fn `Initialize`
  (bind _actor (`/Game/Programming/Entities/BPI_Entity.Get Actor` (`self.Entity`)))
  (bind _output_get (set `self.Actor` _actor))
  (if (not (`Actor.IsActorTickEnabled` _output_get))
    (`/Game/Programming/UI/WBP_ATH_ActionButton.Set Texture` (`self.Action Button`) (`self.Run Image`))))