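; BP_FunctionLibrary_Utils is a utility function library for cursor and location queries.
; GetCursorWorldLocation returns the hit location of a complex Visibility-channel trace under the first player's cursor.
; GetCorrectMousePosition multiplies the viewport mouse position by the viewport scale to compensate for UI scaling.
; GetAverageActorsLocation sums the locations of the given actors and divides by their count to return their midpoint.
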(fn `Get Average Actors Location`
  (params (Actors :type "Array of Actor Object Reference"))
  (returns (Location :type "Vector Structure"))
  (locals (`Total Location` :type "Vector Structure"))
  (bind _total_location (`local.Total Location`))
  ;[1 1 1 0.33] Add all Locations
  (for _array_element Actors
    (set `local.Total Location` (+ (`Actor.K2_GetActorLocation` _array_element) _total_location)))
  ;[1 1 1 0.33] Return Average
  (return (/ _total_location (`KismetArrayLibrary.Array_Length` Actors))))

(fn `Get Correct Mouse Position`
  (returns (`Mouse Position` :type "Vector2D Structure"))
  (bind _returnvalue (`WidgetLayoutLibrary.GetViewportScale` null))
  (bind _returnvalue_2 (`WidgetLayoutLibrary.GetMousePositionOnViewport` null))
  (return (* _returnvalue_2 (`KismetMathLibrary.MakeVector2D` _returnvalue _returnvalue))))

(fn `Get Cursor World Location`
  (returns (Location :type "Vector Structure"))
  (return (`.Location` (`GameplayStatics.BreakHitResult` (`PlayerController.GetHitResultUnderCursorByChannel` (`GameplayStatics.GetPlayerController` null) "TraceTypeQuery1" true)))))