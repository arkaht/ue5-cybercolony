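; Player camera pawn that becomes the view target on BeginPlay and provides panning and zoom with an orthographic camera.
; Each tick, MoveCamera feeds keyboard input and mouse position into GetMovementDirection, intended for screen-edge scrolling, then moves the root relative to spring-arm yaw, optionally scaling speed by zoom.
; The mouse wheel sets a clamped zoom target, smoothed on tick and mapped through a curve to ortho width.
; MoveTo repositions the pawn in XY, keeping its height.
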(event `self.ReceiveBeginPlay`
  ;[1 1 1 0.5] Apply View
  (`self.K2_SetActorRotation` (struct :`Yaw` 90.0))
  (`PlayerController.SetViewTargetWithBlend` (`GameplayStatics.GetPlayerController` 0) self 0.0 "VTBlend_Linear" 0.0 false))

(event `self.ReceiveTick`
  (params (DeltaSeconds :type "Float (single-precision)"))
  ;[0 0.15 1 0.5] Movement
  (`|ExecutionSequence`
    (:`then_0`
      (`self.MoveCamera` DeltaSeconds))
    (:`then_1`
      (set `self.Current Zoom` (`KismetMathLibrary.Lerp` (`self.Current Zoom`) (`self.Target Zoom`) (* DeltaSeconds (`/Game/Programming/Data/PDA_CameraSettings.ZoomSmoothSpeed` (`self.Settings`)))))
      (`self.Apply Zoom`))))

(event `InputAxisKey|MouseWheelAxis`
  (params (AxisValue :type "Float (single-precision)"))
  ;[0 0.15 1 0.5] Zoom
  (set `self.Target Zoom` (`KismetMathLibrary.FClamp` (+ (* (stale `self.ReceiveTick` DeltaSeconds) (* AxisValue -1.0) (`/Game/Programming/Data/PDA_CameraSettings.ZoomSpeed` (`self.Settings`))) (`self.Target Zoom`)))))

(fn `Apply Zoom`
  (`CameraComponent.SetOrthoWidth` (`self.Camera`) (`CurveFloat.GetFloatValue` (`/Game/Programming/Data/PDA_CameraSettings.ZoomScaleCurve` (`self.Settings`)) (`self.Current Zoom`))))

(fn `Move To`
  (params (Position :type "Vector2D Structure"))
  (bind (_returnvalue_x _returnvalue_y _returnvalue_z) (`KismetMathLibrary.BreakVector` (`self.K2_GetActorLocation`)))
  (`self.K2_SetActorLocation` (`KismetMathLibrary.Conv_Vector2DToVector` Position _returnvalue_z)))

(fn `MoveCamera`
  (params (`Delta Time` :type "Float (double-precision)"))
  (locals (mousePos :type "Vector2D Structure"))
  (bind (_returnvalue_x _returnvalue_y) (`KismetMathLibrary.BreakVector2D` (`WidgetLayoutLibrary.GetViewportSize`)))
  (bind _returnvalue (`WidgetLayoutLibrary.GetViewportScale`))
  (bind _settings (`self.Settings`))
  (bind (_mousepos_x _mousepos_y) (`KismetMathLibrary.BreakVector2D` (`local.mousePos`)))
  (bind (_relativerotation_roll _relativerotation_pitch _relativerotation_yaw) (`KismetMathLibrary.BreakRotator` (`SceneComponent.RelativeRotation` (`self.SpringArm`))))
  ;[1 1 1 0.5] Get Mouse Position on Viewport
  (bind _returnvalue_2 (`WidgetLayoutLibrary.GetMousePositionOnViewport`))
  (set `local.mousePos` (* _returnvalue_2 (`KismetMathLibrary.MakeVector2D` _returnvalue _returnvalue)))
  ;[1 1 1 0.5] Apply Movement
  (`SceneComponent.K2_AddRelativeLocation` (`self.DefaultSceneRoot`) (`KismetMathLibrary.GreaterGreater_VectorRotator` (* (`KismetMathLibrary.ClampVectorSize` (`KismetMathLibrary.MakeVector` (`self.Get Movement Direction` (* (`self.GetInputAxisValue`) -1.0) _mousepos_x _returnvalue_x) (`self.Get Movement Direction` (`self.GetInputAxisValue`) _mousepos_y _returnvalue_y)) 0.0 1.0) (* (`/Game/Programming/Data/PDA_CameraSettings.MoveSpeed` _settings) (`KismetMathLibrary.SelectFloat` (`KismetMathLibrary.MapRangeClamped` (`self.Target Zoom`) 0.0 1.0 (`/Game/Programming/Data/PDA_CameraSettings.MinMovementScaleByZoom` _settings) 1.0) 1.0 (`/Game/Programming/Data/PDA_CameraSettings.IsMovementScaledByZoom` _settings)) `Delta Time`)) (`KismetMathLibrary.MakeRotator` 0.0 0.0 _relativerotation_yaw)) false false))

(fn `UserConstructionScript`)