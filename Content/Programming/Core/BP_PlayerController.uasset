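; RTS player controller that adds the ATH widget and handles unit selection, move orders and control groups.
; Left-drag runs the HUD's marquee selection, with Shift adding to the selection, and right-click sends selected units to the cursor through their AI controllers.
; Nine group keys assign the selection with Ctrl, select the group on one tap, or move the camera pawn to its average location on double tap.
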(event `self.ReceiveBeginPlay`
  ;[0.25 0 1 0.33] Attach ATH Widget
  (bind _returnvalue (`|GenericCreateObject` "/Game/Programming/UI/WBP_ATH.WBP_ATH_C"))
  (`UserWidget.AddToViewport` _returnvalue 0)
  ;[1 1 1 0.33] Get Pawn Camera
  (bind _asbp_pawn_camera (cast `/Game/Programming/Core/BP_Pawn_Camera` (`GameplayStatics.GetPlayerPawn` 0)))
  (set `self.Pawn Camera` _asbp_pawn_camera))

(event `Key|LeftControl`
  (params (Key :type "Key Structure"))
  ;[0 0.2667 1 0.33] Read Ctrl Input
  (:`Pressed`
    (set `self.Is Ctrl Hold` true))
  (:`Released`
    (set `self.Is Ctrl Hold` false)))

(event `Key|LeftShift`
  (params (Key :type "Key Structure"))
  ;[0 0.2533 1 0.33] Read Shift Input
  (:`Pressed`
    (set `self.Is Shift Hold` true))
  (:`Released`
    (set `self.Is Shift Hold` false)))

(event `InputAction|SelectionGroup_1`
  (params (Key :type "Key Structure"))
  ;[1 0.6667 0 0.33] Selection Groups
  (:`Pressed`
    (`self.Handle Selection Group Inputs` 0)))

(event `Key|LeftMouseButton`
  (params (Key :type "Key Structure"))
  (bind _returnvalue (`self.GetHUD`))
  ;[1 0.6667 0 0.33] Selection Managment
  (:`Pressed`
    ;;[1 1 1 0.33] Marquee Selection
    (message `/Game/Programming/Core/BPI_Selection.Start Selection` _returnvalue (`self.Selection Classes Filter`)))
  (:`Released`
    (bind _selection (message `/Game/Programming/Core/BPI_Selection.End Selection` _returnvalue))
    ;;[1 1 1 0.33] Shift Selection
    (if (not (`self.Is Shift Hold`))
      (`self.Un Select All Units`))
    (for _array_element _selection
      ;;[1 0.08333 0 0.33] Select Units
      (bind _asbp_character_unit (cast `/Game/Programming/Units/BP_Character_Unit` _array_element))
      (`self.Select Unit` _asbp_character_unit))))

(event `InputAction|SelectionGroup_2`
  (params (Key :type "Key Structure"))
  ;[1 0.6667 0 0.33] Selection Groups
  (:`Pressed`
    (`self.Handle Selection Group Inputs` 1)))

(event `InputAction|SelectionGroup_3`
  (params (Key :type "Key Structure"))
  ;[1 0.6667 0 0.33] Selection Groups
  (:`Pressed`
    (`self.Handle Selection Group Inputs` 2)))

(event `InputAction|SelectionGroup_4`
  (params (Key :type "Key Structure"))
  ;[1 0.6667 0 0.33] Selection Groups
  (:`Pressed`
    (`self.Handle Selection Group Inputs` 3)))

(event `InputAction|SelectionGroup_5`
  (params (Key :type "Key Structure"))
  ;[1 0.6667 0 0.33] Selection Groups
  (:`Pressed`
    (`self.Handle Selection Group Inputs` 4)))

(event `InputAction|SelectionGroup_6`
  (params (Key :type "Key Structure"))
  ;[1 0.6667 0 0.33] Selection Groups
  (:`Pressed`
    (`self.Handle Selection Group Inputs` 5)))

(event `InputAction|SelectionGroup_7`
  (params (Key :type "Key Structure"))
  ;[1 0.6667 0 0.33] Selection Groups
  (:`Pressed`
    (`self.Handle Selection Group Inputs` 6)))

(event `InputAction|SelectionGroup_8`
  (params (Key :type "Key Structure"))
  ;[1 0.6667 0 0.33] Selection Groups
  (:`Pressed`
    (`self.Handle Selection Group Inputs` 7)))

(event `InputAction|SelectionGroup_9`
  (params (Key :type "Key Structure"))
  ;[1 0.6667 0 0.33] Selection Groups
  (:`Pressed`
    (`self.Handle Selection Group Inputs` 8)))

(event `Key|RightMouseButton`
  (params (Key :type "Key Structure"))
  (:`Released`
    ;[1 0.08333 0 0.33] Unit Selection: Move To
    (bind _location (`/Game/Programming/Utils/BPFL_Utils.Get Cursor World Location`))
    (bind _result (`BlueprintSetLibrary.Set_ToArray` (`self.Selected Units`)))
    (for _array_element _result
      (bind _asbp_aicontroller_unit (cast `/Game/Programming/Units/BP_AIController_Unit` (`AIBlueprintHelperLibrary.GetAIController` _array_element)))
      (`/Game/Programming/Units/BP_AIController_Unit.Move To` _asbp_aicontroller_unit _location))))

(fn `Register Unit`
  (params (Unit :type "/Game/Programming/Units/BP_Character_Unit Object Reference"))
  (`BlueprintSetLibrary.Set_Add` (`self.Units`) Unit))

(fn `Select All Units`
  (bind _result (`BlueprintSetLibrary.Set_ToArray` (`self.Units`)))
  (for _array_element _result
    (`self.Select Unit` _array_element)))

(fn `Select Selection Group`
  (params (ID :type Integer))
  (returns (`Is Success` :type Boolean))
  (bind (_value _returnvalue) (`BlueprintMapLibrary.Map_Find` (`self.Selection Groups`) ID))
  (`self.Un Select All Units`)
  (if _returnvalue
    (for _array_element (break `/Game/Programming/Data/S_Array_CharacterUnit` _value)
      (`self.Select Unit` _array_element))
    (return true)
    (else
      (return false))))

(fn `Select Unit`
  (params (Unit :type "/Game/Programming/Units/BP_Character_Unit Object Reference"))
  (bind _selected_units (`self.Selected Units`))
  (if (not (`BlueprintSetLibrary.Set_Contains` _selected_units Unit))
    (`BlueprintSetLibrary.Set_Add` _selected_units Unit)
    (`/Game/Programming/Units/BP_Character_Unit.Set Selected` Unit true)))

(fn `Set Selection Group`
  (params (ID :type Integer) (Units :type "Array of /Game/Programming/Units/BP_Character_Unit Object Reference"))
  (`BlueprintMapLibrary.Map_Add` (`self.Selection Groups`) ID (make `/Game/Programming/Data/S_Array_CharacterUnit` Units)))

(fn `Set Selection Group To Selected`
  (params (ID :type Integer))
  (bind _result (`BlueprintSetLibrary.Set_ToArray` (`self.Selected Units`)))
  (`self.Set Selection Group` ID _result)
  (`self.On Selection Group Changed` ID _result))

(fn `Teleport Camera to Selection Group`
  (params (ID :type Integer))
  (returns (`Is Success` :type Boolean))
  (bind (_value _returnvalue) (`BlueprintMapLibrary.Map_Find` (`self.Selection Groups`) ID))
  ;[1 1 1 0.33] Check Existing Group
  (if _returnvalue
    ;[1 1 1 0.33] Teleport
    (bind _location (`/Game/Programming/Utils/BPFL_Utils.Get Average Actors Location` (break `/Game/Programming/Data/S_Array_CharacterUnit` _value)))
    (`/Game/Programming/Core/BP_Pawn_Camera.Move To` (`self.Pawn Camera`) (`KismetMathLibrary.MakeVector2D` (.x _location) (.y _location)))
    (return true)
    (else
      (return false))))

(fn `Un Register Unit`
  (params (Unit :type "/Game/Programming/Units/BP_Character_Unit Object Reference"))
  (`BlueprintSetLibrary.Set_Remove` (`self.Units`) Unit))

(fn `Un Select All Units`
  (bind _result (`BlueprintSetLibrary.Set_ToArray` (`self.Selected Units`)))
  (for _array_element _result
    (`self.Un Select Unit` _array_element)))

(fn `Un Select Unit`
  (params (Unit :type "/Game/Programming/Units/BP_Character_Unit Object Reference"))
  (`BlueprintSetLibrary.Set_Remove` (`self.Selected Units`) Unit)
  (`/Game/Programming/Units/BP_Character_Unit.Set Selected` Unit false))

(fn `UserConstructionScript`)