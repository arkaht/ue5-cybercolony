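; Character base for selectable units, configured from a row in the DT_Units data table.
; On BeginPlay it registers with BP_PlayerController and unregisters on EndPlay.
; The retrieved row sets walk speed, health, anim class and skeletal mesh at runtime, so the construction script stays empty.
; SetSelected stores the selection state and fires events that show or hide the selection decal.
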(event `self.ReceiveBeginPlay`
  (bind _mesh (`self.Mesh`))
  ;[1 1 1 0.33] Register to Player Controller
  (bind _asbp_player_controller (cast `/Game/Programming/Core/BP_PlayerController` (`GameplayStatics.GetPlayerController` 0)))
  (`/Game/Programming/Core/BP_PlayerController.Register Unit` _asbp_player_controller self)
  ;[1 1 1 0.33] Retrieve Unit Data
  (bind _row (`/Game/Programming/Utils/BPML_ActorUtils.Retrieve Data Table Row` "/Game/Design/Data/DT_Units.DT_Units" (`self.Unit Data Row`))
    (:`Row Found`
      (bind _output_get (set `self.Unit Data` _row))
      ;[1 1 1 0.33] Setup Data
      (set `CharacterMovementComponent.MaxWalkSpeed` (`.MovementSpeed_17_D68F84F440BC524403D18C9AEBAC7497` (break `/Game/Programming/Data/S_UnitData` _output_get)) (`self.CharacterMovement`))
      (set `self.Health` (break `/Game/Programming/Data/S_UnitData` _output_get))
      ;;[1 1 1 0.33] Mesh
      (`SkeletalMeshComponent.SetAnimInstanceClass` _mesh (`.AnimClass_28_4D67512B40E47AD7585FF1BB42203C42` (break `/Game/Programming/Data/S_UnitData` _output_get)))
      (`SkinnedMeshComponent.SetSkinnedAssetAndUpdate` _mesh (`.SkeletalMesh_23_E94D2445496A7F9F1AFDA6B88628238A` (break `/Game/Programming/Data/S_UnitData` _output_get)) true))))

(event `self.ReceiveEndPlay`
  (params (EndPlayReason :type "EEndPlayReason Enum" :default "Destroyed"))
  ;[1 1 1 0.33] Un Register to Player Controller
  (bind _asbp_player_controller (cast `/Game/Programming/Core/BP_PlayerController` (`GameplayStatics.GetPlayerController` 0)))
  (`/Game/Programming/Core/BP_PlayerController.Un Register Unit` _asbp_player_controller self))

(event `OnSelected`
  ;[1 1 1 0.33] Show Selection Decal
  (`SceneComponent.SetVisibility` (`self.DecalSelection`) true false))

(event `OnUnSelected`
  ;[1 1 1 0.33] Hide Selection Decal
  (`SceneComponent.SetVisibility` (`self.DecalSelection`) false false))

(fn `Set Selected`
  (params (`Is Selected` :type Boolean))
  (bind _output_get (set `self.Is Selected` `Is Selected`))
  (if _output_get
    (`self.OnSelected`)
    (else
      (`self.OnUnSelected`))))

(fn `UserConstructionScript`)